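; Parent portal actor for level travel, though every event is an empty stub and the logic below them is disconnected.
; The unwired overlap logic flags the player as within portal range and registers the portal to try.
; The unwired try logic either shows a locked dialogue popup with camera toggle, or stores a spawn point name on the game instance and opens the destination level.
; An unwired end-prompt chain removes the popup and restores walking.
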(event OnComponentBeginOverlap(Box)
  (params (OverlappedComponent :type Primitive%20Component%20Object%20Reference) (OtherActor :type Actor%20Object%20Reference) (OtherComp :type Primitive%20Component%20Object%20Reference) (OtherBodyIndex :type Integer) (bFromSweep :type Boolean) (SweepResult :type Hit%20Result%20Structure%20%28by%20ref%29))
  ;[1 1 1] On Component Begin Overlap (with PC)
)

(event OnComponentEndOverlap(Box)
  (params (OverlappedComponent :type Primitive%20Component%20Object%20Reference) (OtherActor :type Actor%20Object%20Reference) (OtherComp :type Primitive%20Component%20Object%20Reference) (OtherBodyIndex :type Integer))
  ;[1 1 1] On Component End Overlap (with PC)
)

(event Custom|TryPortal
  (params (PortalToTry :type BP%20Portal%20Parent%20Object%20Reference))
  ;[1 1 1] TryPortal
)

(event Custom|End%20Prompt
  ;[1 1 1] End Prompt
)

(event EventBeginPlay)

(event Collision|EventActorBeginOverlap
  (params (OtherActor :type Actor%20Object%20Reference)))

(event EventTick
  (params (DeltaSeconds :type Float%20%28single-precision%29)))

(fn ConstructionScript)