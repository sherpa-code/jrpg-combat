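; BP_CharacterRecorder is a character stand-in in the SceneCaptures folder that registers itself with the yusa3C_BP player on BeginPlay.
; Its weapon update event replaces the back-slot actor with a hard-coded Sword1BP, ignoring NewWeapon.
; AttachItem and UnAttachItem spawn, socket-attach or destroy gear by slot, but the empty equip events leave them disconnected.
; AttachItem's weapon fallback mistakenly attaches the failed tool cast instead of the weapon.
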(event Custom|updateBPCharRecWeapon
  (params (newWeapon :type Weapon%20Parent%20BP%20Object%20Reference))
  (Utilities|IsValid (Variables|Default|GetbackSlot)
    (:Is%20Valid
      (Actor|DestroyActor (Variables|Default|GetbackSlot)))
    (:Is%20Not%20Valid
      _))
  ;[1 1 1] Spawn Sword1 into backSlot
  (bind _returnvalue (Game|SpawnActorfromClass "/Game/0-Project/0-Blueprints/00-ImportedBPs/0Project/Blueprints/weapons/sword1/sword1BP.sword1BP_C" (Transformation|GetSocketTransform (Variables|Default|GetSkeletalMesh) "backSlot" "RTS_World") "Undefined" 0 0))
  (bind _output_get (Variables|Default|SetbackSlot _returnvalue))
  (Transformation|AttachComponentToComponent _output_get (Variables|Default|GetSkeletalMesh) "backSlot" "SnapToTarget" "SnapToTarget" "KeepWorld" true))

(event EventBeginPlay
  (bind _asyusa_3c_bp (Utilities|Casting|CastToyusa3C_BP (Game|GetPlayerCharacter 0)))
  (Class|BPIRecorderComm|PassReference(Message) _asyusa_3c_bp self))

(event Collision|EventActorBeginOverlap
  (params (OtherActor :type Actor%20Object%20Reference)))

(event EventTick
  (params (DeltaSeconds :type Float%20%28single-precision%29)))

(event EventEquipItem
  (params (ItemInfo :type F%20Item%20Info%20Structure)))

(event EventUnEquipItem
  (params (Item%20Info :type F%20Item%20Info%20Structure)))

(fn ConstructionScript)

(fn UnAttachItem
  (params (ItemInfo :type F%20Item%20Info%20Structure))
  (switch Utilities|FlowControl|Switch|SwitchonESlotType (Utilities|Struct|BreakFItemInfo ItemInfo)
    (:NewEnumerator1
      (Actor|DestroyActor (Variables|Default|GetheadItem)))
    (:NewEnumerator2
      (Actor|DestroyActor (Variables|Default|GettorsoItem)))
    (:NewEnumerator3
      (Actor|DestroyActor (Variables|Default|GetarmsItem)))
    (:NewEnumerator10
      (Actor|DestroyActor (Variables|Default|GetlegsItem)))
    (:NewEnumerator11
      (Actor|DestroyActor (Variables|Default|GetfeetItem)))
    (:NewEnumerator5
      (Actor|DestroyActor (Variables|Default|GetPrimaryRightHandItem) :!label _label))
    (:NewEnumerator12
      (goto _label))
    (:NewEnumerator6
      (Actor|DestroyActor (Variables|Default|GetPrimaryLeftHandItem)))
    (:NewEnumerator7
      (Actor|DestroyActor (Variables|Default|GetSecondaryRightHandItem)))
    (:NewEnumerator8
      (Actor|DestroyActor (Variables|Default|GetSecondaryLeftHandItem)))
    (:NewEnumerator9
      (Actor|DestroyActor (Variables|Default|GetAmuletItem)))))

(fn AttachItem
  (params (ItemInfo :type F%20Item%20Info%20Structure))
  (bind (_itemclass _itemslot) (Utilities|Struct|BreakFItemInfo ItemInfo))
  (switch Utilities|FlowControl|Switch|SwitchonESlotType _itemslot
    (:NewEnumerator1
      (Utilities|IsValid (Variables|Default|GetheadItem)
        (:Is%20Valid
          (Actor|DestroyActor (Variables|Default|GetheadItem)))
        (:Is%20Not%20Valid
          _))
      (bind _returnvalue (Game|SpawnActorfromClass _itemclass (Transformation|GetActorTransform) "AlwaysSpawn" 0 0))
      (bind _output_get (Variables|Default|SetheadItem _returnvalue))
      (bind _asbp_base_wearable (Utilities|Casting|CastToBP_BaseWearable _output_get))
      (Transformation|AttachComponentToComponent _asbp_base_wearable (Variables|Default|GetSkeletalMesh) (.HeadSlot (Utilities|Struct|BreakFWearableInfo (Variables|/Game/0-Project/0-Blueprints/00-ImportedBPs/0Project/Blueprints/Interactables/Wearable/BP_BaseWearable.BP_BaseWearable_C|GetWearableInfo _asbp_base_wearable))) "SnapToTarget" "SnapToTarget" "SnapToTarget" true)
      (Collision|SetActorEnableCollision _asbp_base_wearable false))
    (:NewEnumerator2
      (Utilities|IsValid (Variables|Default|GettorsoItem)
        (:Is%20Valid
          (Actor|DestroyActor (Variables|Default|GettorsoItem)))
        (:Is%20Not%20Valid
          _))
      (bind _returnvalue_2 (Game|SpawnActorfromClass _itemclass (Transformation|GetActorTransform) "AlwaysSpawn" 0 0))
      (bind _output_get_2 (Variables|Default|SettorsoItem _returnvalue_2))
      (bind _asbp_base_wearable_2 (Utilities|Casting|CastToBP_BaseWearable _output_get_2))
      (Transformation|AttachComponentToComponent _asbp_base_wearable_2 (Variables|Default|GetSkeletalMesh) (.ChestSlot (Utilities|Struct|BreakFWearableInfo (Variables|/Game/0-Project/0-Blueprints/00-ImportedBPs/0Project/Blueprints/Interactables/Wearable/BP_BaseWearable.BP_BaseWearable_C|GetWearableInfo _asbp_base_wearable_2))) "SnapToTarget" "SnapToTarget" "SnapToTarget" true)
      (Collision|SetActorEnableCollision _asbp_base_wearable_2 false))
    (:NewEnumerator3
      (Utilities|IsValid (Variables|Default|GetarmsItem)
        (:Is%20Valid
          (Actor|DestroyActor (Variables|Default|GetarmsItem)))
        (:Is%20Not%20Valid
          _))
      (bind _returnvalue_3 (Game|SpawnActorfromClass _itemclass (Transformation|GetActorTransform) "AlwaysSpawn" 0 0))
      (bind _output_get_3 (Variables|Default|SetarmsItem _returnvalue_3))
      (bind _asbp_base_wearable_3 (Utilities|Casting|CastToBP_BaseWearable _output_get_3))
      (Transformation|AttachComponentToComponent _asbp_base_wearable_3 (Variables|Default|GetSkeletalMesh) (.ArmSlot (Utilities|Struct|BreakFWearableInfo (Variables|/Game/0-Project/0-Blueprints/00-ImportedBPs/0Project/Blueprints/Interactables/Wearable/BP_BaseWearable.BP_BaseWearable_C|GetWearableInfo _asbp_base_wearable_3))) "SnapToTarget" "SnapToTarget" "SnapToTarget" true)
      (Collision|SetActorEnableCollision _asbp_base_wearable_3 false))
    (:NewEnumerator10
      (Utilities|IsValid (Variables|Default|GetlegsItem)
        (:Is%20Valid
          (Actor|DestroyActor (Variables|Default|GetlegsItem)))
        (:Is%20Not%20Valid
          _))
      (bind _returnvalue_4 (Game|SpawnActorfromClass _itemclass (Transformation|GetActorTransform) "AlwaysSpawn" 0 0))
      (bind _output_get_4 (Variables|Default|SetlegsItem _returnvalue_4))
      (bind _asbp_base_wearable_4 (Utilities|Casting|CastToBP_BaseWearable _output_get_4))
      (Transformation|AttachComponentToComponent _asbp_base_wearable_4 (Variables|Default|GetSkeletalMesh) (.LegSlot (Utilities|Struct|BreakFWearableInfo (Variables|/Game/0-Project/0-Blueprints/00-ImportedBPs/0Project/Blueprints/Interactables/Wearable/BP_BaseWearable.BP_BaseWearable_C|GetWearableInfo _asbp_base_wearable_4))) "SnapToTarget" "SnapToTarget" "SnapToTarget" true)
      (Collision|SetActorEnableCollision _asbp_base_wearable_4 false))
    (:NewEnumerator11
      (Utilities|IsValid (Variables|Default|GetfeetItem)
        (:Is%20Valid
          (Actor|DestroyActor (Variables|Default|GetfeetItem)))
        (:Is%20Not%20Valid
          _))
      (bind _returnvalue_5 (Game|SpawnActorfromClass _itemclass (Transformation|GetActorTransform) "AlwaysSpawn" 0 0))
      (bind _output_get_5 (Variables|Default|SetfeetItem _returnvalue_5))
      (bind _asbp_base_wearable_5 (Utilities|Casting|CastToBP_BaseWearable _output_get_5))
      (Transformation|AttachComponentToComponent _asbp_base_wearable_5 (Variables|Default|GetSkeletalMesh) (.FeetSlot (Utilities|Struct|BreakFWearableInfo (Variables|/Game/0-Project/0-Blueprints/00-ImportedBPs/0Project/Blueprints/Interactables/Wearable/BP_BaseWearable.BP_BaseWearable_C|GetWearableInfo _asbp_base_wearable_5))) "SnapToTarget" "SnapToTarget" "SnapToTarget" true)
      (Collision|SetActorEnableCollision _asbp_base_wearable_5 false))
    (:NewEnumerator5
      (Utilities|IsValid (Variables|Default|GetPrimaryRightHandItem)
        (:Is%20Valid
          (Actor|DestroyActor (Variables|Default|GetPrimaryRightHandItem)))
        (:Is%20Not%20Valid
          _))
      (bind _returnvalue_6 (Game|SpawnActorfromClass _itemclass (Transformation|GetActorTransform) "AlwaysSpawn" 0 0))
      (bind _output_get_6 (Variables|Default|SetPrimaryRightHandItem _returnvalue_6))
      (bind _asbp_base_tool (Utilities|Casting|CastToBP_BaseTool _output_get_6)
        (:then
          (Development|PrintString (Utilities|String|ToString(Name) (.PrimaryRightHand (Utilities|Struct|BreakFToolInfo (Variables|/Game/0-Project/0-Blueprints/00-ImportedBPs/0Project/Blueprints/Interactables/Tools/BP_BaseTool.BP_BaseTool_C|GetToolInfo _asbp_base_tool)))))
          (Transformation|AttachComponentToComponent _asbp_base_tool (Variables|Default|GetSkeletalMesh) (.PrimaryRightHand (Utilities|Struct|BreakFToolInfo (Variables|/Game/0-Project/0-Blueprints/00-ImportedBPs/0Project/Blueprints/Interactables/Tools/BP_BaseTool.BP_BaseTool_C|GetToolInfo _asbp_base_tool))) "SnapToTarget" "SnapToTarget" "SnapToTarget" true)
          (Development|PrintString "Hello")
          (Collision|SetActorEnableCollision _asbp_base_tool false))
        (:CastFailed
          (Development|PrintString "toolfail")
          (bind _asbp_base_weapon (Utilities|Casting|CastToBP_BaseWeapon _output_get_6))
          (Transformation|AttachComponentToComponent _asbp_base_tool (Variables|Default|GetSkeletalMesh) (Utilities|Struct|BreakFWeaponInfo (Variables|/Game/0-Project/0-Blueprints/00-ImportedBPs/0Project/Blueprints/Interactables/Weapons/BP_BaseWeapon.BP_BaseWeapon_C|GetWeaponInfo _asbp_base_weapon)) "SnapToTarget" "SnapToTarget" "SnapToTarget" true)
          (Collision|SetActorEnableCollision _asbp_base_tool false))))
    (:NewEnumerator12
      (Utilities|IsValid (Variables|Default|GetPrimaryRightHandItem)
        (:Is%20Valid
          (Actor|DestroyActor (Variables|Default|GetPrimaryRightHandItem)))
        (:Is%20Not%20Valid
          _))
      (bind _returnvalue_7 (Game|SpawnActorfromClass _itemclass (Transformation|GetActorTransform) "AlwaysSpawn" 0 0))
      (bind _output_get_7 (Variables|Default|SetPrimaryRightHandItem _returnvalue_7))
      (bind _asbp_base_tool_2 (Utilities|Casting|CastToBP_BaseTool _output_get_7)
        (:then
          (Development|PrintString (Utilities|String|ToString(Name) (Utilities|Struct|BreakFToolInfo (Variables|/Game/0-Project/0-Blueprints/00-ImportedBPs/0Project/Blueprints/Interactables/Tools/BP_BaseTool.BP_BaseTool_C|GetToolInfo _asbp_base_tool_2))))
          (Transformation|AttachComponentToComponent _asbp_base_tool_2 (Variables|Default|GetSkeletalMesh) (Utilities|Struct|BreakFToolInfo (Variables|/Game/0-Project/0-Blueprints/00-ImportedBPs/0Project/Blueprints/Interactables/Tools/BP_BaseTool.BP_BaseTool_C|GetToolInfo _asbp_base_tool_2)) "SnapToTarget" "SnapToTarget" "SnapToTarget" true)
          (Development|PrintString "Hello")
          (Collision|SetActorEnableCollision _asbp_base_tool_2 false))
        (:CastFailed
          (Development|PrintString "toolfail")
          (bind _asbp_base_weapon_2 (Utilities|Casting|CastToBP_BaseWeapon _output_get_7))
          (Transformation|AttachComponentToComponent _asbp_base_tool_2 (Variables|Default|GetSkeletalMesh) (Utilities|Struct|BreakFWeaponInfo (Variables|/Game/0-Project/0-Blueprints/00-ImportedBPs/0Project/Blueprints/Interactables/Weapons/BP_BaseWeapon.BP_BaseWeapon_C|GetWeaponInfo _asbp_base_weapon_2)) "SnapToTarget" "SnapToTarget" "SnapToTarget" true)
          (Collision|SetActorEnableCollision _asbp_base_tool_2 false))))
    (:NewEnumerator6
      (Utilities|IsValid (Variables|Default|GetPrimaryLeftHandItem)
        (:Is%20Valid
          (Actor|DestroyActor (Variables|Default|GetPrimaryLeftHandItem)))
        (:Is%20Not%20Valid
          _))
      (bind _returnvalue_8 (Game|SpawnActorfromClass _itemclass (Transformation|GetActorTransform) "AlwaysSpawn" 0 0))
      (bind _output_get_8 (Variables|Default|SetPrimaryLeftHandItem _returnvalue_8))
      (bind _asbp_base_tool_3 (Utilities|Casting|CastToBP_BaseTool _output_get_8)
        (:then
          (Transformation|AttachComponentToComponent _asbp_base_tool_3 (Variables|Default|GetSkeletalMesh) (.PrimaryLeftHand (Utilities|Struct|BreakFToolInfo (Variables|/Game/0-Project/0-Blueprints/00-ImportedBPs/0Project/Blueprints/Interactables/Tools/BP_BaseTool.BP_BaseTool_C|GetToolInfo _asbp_base_tool_3))) "SnapToTarget" "SnapToTarget" "SnapToTarget" true)
          (Collision|SetActorEnableCollision _asbp_base_tool_3 false))
        (:CastFailed
          (bind _asbp_base_weapon_3 (Utilities|Casting|CastToBP_BaseWeapon _output_get_8))
          (Transformation|AttachComponentToComponent _asbp_base_tool_3 (Variables|Default|GetSkeletalMesh) (Utilities|Struct|BreakFWeaponInfo (Variables|/Game/0-Project/0-Blueprints/00-ImportedBPs/0Project/Blueprints/Interactables/Weapons/BP_BaseWeapon.BP_BaseWeapon_C|GetWeaponInfo _asbp_base_weapon_3)) "SnapToTarget" "SnapToTarget" "SnapToTarget" true)
          (Collision|SetActorEnableCollision _asbp_base_tool_3 false))))
    (:NewEnumerator7
      (Utilities|IsValid (Variables|Default|GetSecondaryRightHandItem)
        (:Is%20Valid
          (Actor|DestroyActor (Variables|Default|GetSecondaryRightHandItem)))
        (:Is%20Not%20Valid
          _))
      (bind _returnvalue_9 (Game|SpawnActorfromClass _itemclass (Transformation|GetActorTransform) "AlwaysSpawn" 0 0))
      (bind _output_get_9 (Variables|Default|SetSecondaryRightHandItem _returnvalue_9))
      (bind _asbp_base_tool_4 (Utilities|Casting|CastToBP_BaseTool _output_get_9)
        (:then
          (Transformation|AttachComponentToComponent _asbp_base_tool_4 (Variables|Default|GetSkeletalMesh) (.SecondaryRightHand (Utilities|Struct|BreakFToolInfo (Variables|/Game/0-Project/0-Blueprints/00-ImportedBPs/0Project/Blueprints/Interactables/Tools/BP_BaseTool.BP_BaseTool_C|GetToolInfo _asbp_base_tool_4))) "SnapToTarget" "SnapToTarget" "SnapToTarget" true)
          (Collision|SetActorEnableCollision _asbp_base_tool_4 false))
        (:CastFailed
          (bind _asbp_base_weapon_4 (Utilities|Casting|CastToBP_BaseWeapon _output_get_9))
          (Transformation|AttachComponentToComponent _asbp_base_tool_4 (Variables|Default|GetSkeletalMesh) (Utilities|Struct|BreakFWeaponInfo (Variables|/Game/0-Project/0-Blueprints/00-ImportedBPs/0Project/Blueprints/Interactables/Weapons/BP_BaseWeapon.BP_BaseWeapon_C|GetWeaponInfo _asbp_base_weapon_4)) "SnapToTarget" "SnapToTarget" "SnapToTarget" true)
          (Collision|SetActorEnableCollision _asbp_base_tool_4 false))))
    (:NewEnumerator8
      (Utilities|IsValid (Variables|Default|GetSecondaryLeftHandItem)
        (:Is%20Valid
          (Actor|DestroyActor (Variables|Default|GetSecondaryLeftHandItem)))
        (:Is%20Not%20Valid
          _))
      (bind _returnvalue_10 (Game|SpawnActorfromClass _itemclass (Transformation|GetActorTransform) "AlwaysSpawn" 0 0))
      (bind _output_get_10 (Variables|Default|SetSecondaryLeftHandItem _returnvalue_10))
      (bind _asbp_base_tool_5 (Utilities|Casting|CastToBP_BaseTool _output_get_10)
        (:then
          (Transformation|AttachComponentToComponent _asbp_base_tool_5 (Variables|Default|GetSkeletalMesh) (.SecondaryLeftHand (Utilities|Struct|BreakFToolInfo (Variables|/Game/0-Project/0-Blueprints/00-ImportedBPs/0Project/Blueprints/Interactables/Tools/BP_BaseTool.BP_BaseTool_C|GetToolInfo _asbp_base_tool_5))) "SnapToTarget" "SnapToTarget" "SnapToTarget" true)
          (Collision|SetActorEnableCollision _asbp_base_tool_5 false))
        (:CastFailed
          (bind _asbp_base_weapon_5 (Utilities|Casting|CastToBP_BaseWeapon _output_get_10))
          (Transformation|AttachComponentToComponent _asbp_base_tool_5 (Variables|Default|GetSkeletalMesh) (Utilities|Struct|BreakFWeaponInfo (Variables|/Game/0-Project/0-Blueprints/00-ImportedBPs/0Project/Blueprints/Interactables/Weapons/BP_BaseWeapon.BP_BaseWeapon_C|GetWeaponInfo _asbp_base_weapon_5)) "SnapToTarget" "SnapToTarget" "SnapToTarget" true)
          (Collision|SetActorEnableCollision _asbp_base_tool_5 false))))
    (:NewEnumerator9
      (Utilities|IsValid (Variables|Default|GetAmuletItem)
        (:Is%20Valid
          (Actor|DestroyActor (Variables|Default|GetAmuletItem)))
        (:Is%20Not%20Valid
          _))
      (bind _returnvalue_11 (Game|SpawnActorfromClass _itemclass (Transformation|GetActorTransform) "AlwaysSpawn" 0 0))
      (bind _output_get_11 (Variables|Default|SetAmuletItem _returnvalue_11))
      (bind _asbp_base_wearable_6 (Utilities|Casting|CastToBP_BaseWearable _output_get_11))
      (Transformation|AttachComponentToComponent _asbp_base_wearable_6 (Variables|Default|GetSkeletalMesh) (.AttachPoint (Utilities|Struct|BreakFWearableInfo (Variables|/Game/0-Project/0-Blueprints/00-ImportedBPs/0Project/Blueprints/Interactables/Wearable/BP_BaseWearable.BP_BaseWearable_C|GetWearableInfo _asbp_base_wearable_6))) "SnapToTarget" "SnapToTarget" "SnapToTarget" true)
      (Collision|SetActorEnableCollision _asbp_base_wearable_6 false))))