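; BP_BaseItem is a base interactable pickup item actor that can be collected into an inventory.
; The construction script rebuilds ItemInfo with the actor's own class written into it, keeping the other fields as set.
; On Interaction, it checks whether the instigator has inventory space, and if so passes ItemInfo through PickupMessage and destroys itself.
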(event EventBeginPlay
  (|CallParentFunction))

(event Collision|EventActorBeginOverlap
  (params (OtherActor :type Actor%20Object%20Reference))
  (|CallParentFunction OtherActor))

(event EventTick
  (params (DeltaSeconds :type Float%20%28single-precision%29))
  (|CallParentFunction DeltaSeconds))

(event EventInteraction
  (params (Instigator :type Char%201%20Object%20Reference))
  (if (Default|HasSpaceinInventory Instigator)
    (Class|BPIInteract|Pickup(Message) Instigator (Variables|Default|GetItemInfo))
    (Actor|DestroyActor)))

(fn ConstructionScript
  (|CallParentFunction)
  (Variables|Default|SetItemInfo (Utilities|Struct|MakeFItemInfo (.itemtype (Variables|Default|GetItemInfo)) (.itemname (Variables|Default|GetItemInfo)) (.itemimage (Variables|Default|GetItemInfo)) (Utilities|GetClass self) (.itemindex (Variables|Default|GetItemInfo)) (.itemslot (Variables|Default|GetItemInfo)) (.itemvalue (Variables|Default|GetItemInfo)))))