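; Portal base Blueprint for doors that move the player between Chapter 1 levels or show a locked message.
; Box overlap registers the portal on the player character as PortalToTry.
; TryPortal disables movement, then either sets a spawn point name in the game instance and opens the destination level, or opens a camera and "It's locked." dialogue.
; The locked branch polls for dialogue completion with a Delay loop before EndPrompt restores control.
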(event OnComponentBeginOverlap(Box)
  (params (OverlappedComponent :type Primitive%20Component%20Object%20Reference) (OtherActor :type Actor%20Object%20Reference) (OtherComp :type Primitive%20Component%20Object%20Reference) (OtherBodyIndex :type Integer) (bFromSweep :type Boolean) (SweepResult :type Hit%20Result%20Structure%20%28by%20ref%29))
  (bind _pcreference (Variables|Default|GetPCReference))
  ;[1 1 1] On Component Begin Overlap (with PC)
  (bind _asyusa_3c_bp (Utilities|Casting|CastToyusa3C_BP OtherActor))
  (if (not (Variables|/Game/0-Project/0-Blueprints/00-ImportedBPs/0Project/Blueprints/PCs/CharC_delta/yusa3C_BP.yusa3C_BP_C|GetisWithinPortalRange _asyusa_3c_bp))
    (Utilities|IsValid _pcreference
      (:Is%20Valid
        (Variables|/Game/0-Project/0-Blueprints/00-ImportedBPs/0Project/Blueprints/PCs/CharC_delta/yusa3C_BP.yusa3C_BP_C|SetisWithinPortalRange _pcreference true)
        (Development|PrintString "Hello")
        (Variables|/Game/0-Project/0-Blueprints/00-ImportedBPs/0Project/Blueprints/PCs/CharC_delta/yusa3C_BP.yusa3C_BP_C|SetportalToTry (Variables|Default|GetPCReference) self)))))

(event OnComponentEndOverlap(Box)
  (params (OverlappedComponent :type Primitive%20Component%20Object%20Reference) (OtherActor :type Actor%20Object%20Reference) (OtherComp :type Primitive%20Component%20Object%20Reference) (OtherBodyIndex :type Integer))
  ;[1 1 1] On Component End Overlap (with PC)
  (bind _asyusa_3c_bp (Utilities|Casting|CastToyusa3C_BP OtherActor))
  (Utilities|IsValid (Variables|/Game/0-Project/0-Blueprints/00-ImportedBPs/0Project/Blueprints/PCs/CharC_delta/yusa3C_BP.yusa3C_BP_C|GetportalToTry _asyusa_3c_bp)
    (:Is%20Valid
      (Variables|/Game/0-Project/0-Blueprints/00-ImportedBPs/0Project/Blueprints/PCs/CharC_delta/yusa3C_BP.yusa3C_BP_C|SetisWithinPortalRange (Variables|Default|GetPCReference) false)
      (Development|PrintString "Bye")
      (Variables|/Game/0-Project/0-Blueprints/00-ImportedBPs/0Project/Blueprints/PCs/CharC_delta/yusa3C_BP.yusa3C_BP_C|SetportalToTry (Variables|Default|GetPCReference) 0))))

(event Custom|TryPortal
  (params (PortalToTry :type BP%20Portal%20Parent%20Object%20Reference))
  ;[1 1 1] TryPortal
  (Pawn|Components|CharacterMovement|DisableMovement (Variables|/Script/Engine.Character|GetCharacterMovement (Variables|Default|GetPCReference)))
  (if (Variables|Default|GetisLocked)
    (Default|InteractableCameraOpenClose (Variables|Default|GetPCReference) self "NewEnumerator0")
    ;[0.5529 1 0.3216] 'Is Locked' Popup (Talk method - Create)
    ;;[1 1 1] Create widget (fade in)
    (Default|DialoguePopupCreate (Variables|Default|GetPCReference) "NewEnumerator0" "NewEnumerator0" "NewEnumerator0" "NewEnumerator2" "NewEnumerator0" 0 self)
    ;;[1 1 1] Add scripts, print
    (Default|DialoguePopupAddScripts (Variables|Default|GetPCReference) "" "" (Utilities|Array|MakeArray "It's locked."))
    (Default|DialoguePopupClearandPrintScript (Variables|Default|GetPCReference) "NewEnumerator0")
    ;;[1 1 1] Wait for dialogue completion
    (if (Variables|Default|GetisDialogueComplete?) :!label _label
      ;[1 1 1] End Prompt
      (CallFunction|EndPrompt)
      (else
        (Utilities|FlowControl|Delay 0.6)
        (goto _label)))
    (else
      (switch Utilities|FlowControl|Switch|SwitchonE_Level (Variables|Default|GetDestination_Level)
        (:NewEnumerator1
          (switch Utilities|FlowControl|Switch|SwitchonE_Ardence_Spawns (Variables|Default|GetArdence_SpawnPoint)
            (:NewEnumerator1
              (bind _asmy_game_instance (Utilities|Casting|CastToMyGameInstance (Game|GetGameInstance)))
              (Variables|/Game/0-Project/0-Blueprints/00-ImportedBPs/0Project/0-Blueprints/MyGameInstance.MyGameInstance_C|SetTarget_Spawn_DisplayName _asmy_game_instance "BP_ZeinHome_FrontDoor_Ext_SpawnPoint")
              (Game|OpenLevel(byName) "village_1"))
            (:NewEnumerator4
              (bind _asmy_game_instance_2 (Utilities|Casting|CastToMyGameInstance (Game|GetGameInstance)))
              (Variables|/Game/0-Project/0-Blueprints/00-ImportedBPs/0Project/0-Blueprints/MyGameInstance.MyGameInstance_C|SetTarget_Spawn_DisplayName _asmy_game_instance_2 "BP_GlaxShop_FrontDoor_Ext_SpawnPoint")
              (Game|OpenLevel(byName) "village_1"))))
        (:NewEnumerator0
          (bind _asmy_game_instance_3 (Utilities|Casting|CastToMyGameInstance (Game|GetGameInstance)))
          (Variables|/Game/0-Project/0-Blueprints/00-ImportedBPs/0Project/0-Blueprints/MyGameInstance.MyGameInstance_C|SetTarget_Spawn_DisplayName _asmy_game_instance_3 "DefaultTeleportLocation")
          (Game|OpenLevel(byName) "CH01-ZeinHome"))
        (:NewEnumerator2
          (bind _asmy_game_instance_4 (Utilities|Casting|CastToMyGameInstance (Game|GetGameInstance)))
          (Variables|/Game/0-Project/0-Blueprints/00-ImportedBPs/0Project/0-Blueprints/MyGameInstance.MyGameInstance_C|SetTarget_Spawn_DisplayName _asmy_game_instance_4 "DefaultTeleportLocation")
          (Game|OpenLevel(byName) "CH01-GlaxShop"))
        (:NewEnumerator3
          (bind _asmy_game_instance_5 (Utilities|Casting|CastToMyGameInstance (Game|GetGameInstance)))
          (Variables|/Game/0-Project/0-Blueprints/00-ImportedBPs/0Project/0-Blueprints/MyGameInstance.MyGameInstance_C|SetTarget_Spawn_DisplayName _asmy_game_instance_5 "DefaultTeleportLocation")
          (Game|OpenLevel(byName) "CH01-BraxShop"))))))

(event Custom|End%20Prompt
  ;[1 1 1] End Prompt
  ;[1 1 1] DEBUG
  (Development|PrintString "End Prompt")
  (Default|InteractableCameraOpenClose (Variables|Default|GetPCReference) self "NewEnumerator0")
  (Widget|RemovefromParent (Variables|/Game/0-Project/0-Blueprints/00-ImportedBPs/0Project/Blueprints/PCs/CharC_delta/yusa3C_BP.yusa3C_BP_C|GetdialoguePopRef_current (Variables|Default|GetPCReference)))
  (Utilities|FlowControl|Delay 0.25)
  (Variables|/Game/0-Project/0-Blueprints/00-ImportedBPs/0Project/Blueprints/PCs/CharC_delta/yusa3C_BP.yusa3C_BP_C|SetisAnyDiagPopOpen? (Variables|Default|GetPCReference) false)
  (Input|SetInputModeGameOnly (Game|GetPlayerController 0))
  (Pawn|Components|CharacterMovement|SetMovementMode (Variables|/Script/Engine.Character|GetCharacterMovement (Variables|Default|GetPCReference)) "MOVE_Walking" 0))

(event EventBeginPlay
  (bind _asyusa_3c_bp (Utilities|Casting|CastToyusa3C_BP (Game|GetPlayerCharacter 0)))
  (Variables|Default|SetPCReference _asyusa_3c_bp))

(event Collision|EventActorBeginOverlap
  (params (OtherActor :type Actor%20Object%20Reference)))

(event EventTick
  (params (DeltaSeconds :type Float%20%28single-precision%29)))

(fn ConstructionScript)