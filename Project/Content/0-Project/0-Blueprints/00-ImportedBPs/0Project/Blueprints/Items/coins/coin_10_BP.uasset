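; Coin pickup item worth 10 that scatters when it spawns and spins in place about its vertical axis.
; BeginPlay sets the value, spin rate and bouncing Projectile Movement, with a random horizontal velocity scaled by SpawnMovementStrength.
; Tick applies the frame-rate-independent yaw rotation.
; Mesh overlap with the player's yusa3C_BP capsule calls CoinPickup, which is defined outside these graphs.
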(event OnComponentBeginOverlap(StaticMesh_0)
  (params (OverlappedComponent :type Primitive%20Component%20Object%20Reference) (OtherActor :type Actor%20Object%20Reference) (OtherComp :type Primitive%20Component%20Object%20Reference) (OtherBodyIndex :type Integer) (bFromSweep :type Boolean) (SweepResult :type Hit%20Result%20Structure%20%28by%20ref%29)))

(event OnComponentBeginOverlap(StaticMesh)
  (params (OverlappedComponent :type Primitive%20Component%20Object%20Reference) (OtherActor :type Actor%20Object%20Reference) (OtherComp :type Primitive%20Component%20Object%20Reference) (OtherBodyIndex :type Integer) (bFromSweep :type Boolean) (SweepResult :type Hit%20Result%20Structure%20%28by%20ref%29))
  (bind _asyusa_3c_bp (Utilities|Casting|CastToyusa3C_BP (Game|GetPlayerCharacter 0)))
  (if (== (Variables|/Script/Engine.Character|GetCapsuleComponent _asyusa_3c_bp) OtherComp)
    (CallFunction|CoinPickup)))

(event EventBeginPlay
  (bind _spawnmovementstrength (Variables|Default|GetspawnMovementStrength))
  (bind _spawnmovementstrength_2 (Variables|Default|GetspawnMovementStrength))
  (bind _projectilemovement (Variables|Default|GetProjectileMovement))
  (Variables|Default|SetcoinValue 10)
  (Variables|Default|SetyawPerSecond 9e+01)
  ;[1 1 1] Projectile Movement component default values
  (Variables|/Script/Engine.ProjectileMovementComponent|SetInitialSpeed _projectilemovement 1.0)
  (Variables|/Script/Engine.ProjectileMovementComponent|SetProjectileGravityScale _projectilemovement 0.85)
  (Variables|/Script/Engine.ProjectileMovementComponent|SetbShouldBounce _projectilemovement true)
  (Variables|/Script/Engine.MovementComponent|SetVelocity _projectilemovement (Math|Vector|MakeVector (Math|Random|RandomFloatinRange (* -1 _spawnmovementstrength) _spawnmovementstrength) (Math|Random|RandomFloatinRange (* -1 _spawnmovementstrength_2) _spawnmovementstrength_2) 0.0)))

(event EventTick
  (params (DeltaSeconds :type Float%20%28single-precision%29))
  (Class|Actor|AddActorWorldRotation (Math|Rotator|MakeRotator 0.0 0.0 (* DeltaSeconds (Variables|Default|GetyawPerSecond)))))

(fn ConstructionScript)