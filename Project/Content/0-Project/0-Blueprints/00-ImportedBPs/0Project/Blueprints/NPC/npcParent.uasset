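; Base NPC Blueprint that routes interaction and dialogue calls to specific NPC child Blueprints.
; Enum switches cast self to the child: interaction reaches Zein Relwof or Glax Bee, while dialogue handler and continue redirects cover only Zein.
; Damage, death and crosshair events are empty, with their enemy-style logic left disconnected.
; Helper functions remain for dropping coins by denomination and updating the HP widget.
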(event Custom|damageCalcApply
  (params (weaponRef :type Actor%20Object%20Reference) (actorHit :type Actor%20Object%20Reference) (damageTaken :type Integer) (damageType :type String) (lastHitChained :type Integer) (stunAmount :type Integer))
  ;[1 1 1] damageCalcApply (to self)
)

(event Custom|Death
  (params (enemyMesh :type Skeletal%20Mesh%20Component%20Object%20Reference))
  ;[1 1 1] Death
  ;;[1 1 1] Death
)

(event Custom|destroyPointLight
  (params (Owner :type Actor%20Object%20Reference) (toDestroy :type Point%20Light%20Component%20Object%20Reference) (delay :type Float%20%28single-precision%29))
  ;[1 1 1] destroyPointLight
)

(event Custom|deathAnimEnd
  ;[1 1 1] Death
  ;;[1 1 1] deathAnimEnd
)

(event Custom|NPCParent_Interact_Switch
  (params (NPC :type ENPC%20Enum :default "NewEnumerator0"))
  ;[1 1 1] NPCParent Interact Switch
  (switch Utilities|FlowControl|Switch|SwitchonENPC NPC
    (:NewEnumerator0
      (bind _asnpc_a0_bp (Utilities|Casting|CastToNPC_A0_BP self))
      (Default|NPCInteract _asnpc_a0_bp))
    (:NewEnumerator3
      (bind _asnpc_a4_bp (Utilities|Casting|CastToNPC_A4_BP self))
      (Default|NPCInteract _asnpc_a4_bp))))

(event Custom|dialogueHandler_Redirect
  (params (Method :type E_dialogueHandlerMethod%20Enum :default "NewEnumerator0"))
  ;[1 1 1] dialogueHandler_Redirect
  (switch Utilities|FlowControl|Switch|SwitchonENPC (Variables|Default|GetENPC)
    (:NewEnumerator0
      (bind _asnpc_a0_bp (Utilities|Casting|CastToNPC_A0_BP self))
      (Default|DialogueHandler _asnpc_a0_bp Method))))

(event Custom|setCrosshairVisbility
  (params (Input :type Boolean))
  ;[1 1 1] setCrosshairVisibility
)

(event Custom|dialogueContinue_Redirect
  (params (Method :type E_dialogueHandlerMethod%20Enum :default "NewEnumerator0"))
  ;[1 1 1] dialogueContinue_Redirect
  (switch Utilities|FlowControl|Switch|SwitchonENPC (Variables|Default|GetENPC)
    (:NewEnumerator0
      (bind _asnpc_a0_bp (Utilities|Casting|CastToNPC_A0_BP self))
      (Default|DialogueContinue _asnpc_a0_bp Method))))

(fn ConstructionScript)

(fn DropCoins
  (bind _capsulecomponent (Variables|Default|GetCapsuleComponent))
  (bind _returnvalue (Transformation|GetWorldLocation _capsulecomponent))
  (if (>= (/ (Variables|Default|GetcoinsHolding) 500) 1)
    (for _index (range 1 (/ (Variables|Default|GetcoinsHolding) 500))
      (Game|SpawnActorfromClass "/Game/0-Project/0-Blueprints/00-ImportedBPs/0Project/Blueprints/Items/coins/coin_500_bp2.coin_500_bp2_C" (Math|Transform|MakeTransform _returnvalue "0, 0, 0" "0.025000,0.025000,0.025000") "Undefined" 0 0))
    (Variables|Default|SetcoinsHolding (- (Variables|Default|GetcoinsHolding) (* 500 (/ (Variables|Default|GetcoinsHolding) 500)))))
  (if (> (/ (Variables|Default|GetcoinsHolding) 100) 0)
    (for _index_2 (range 1 (/ (Variables|Default|GetcoinsHolding) 100))
      (Game|SpawnActorfromClass "/Game/0-Project/0-Blueprints/00-ImportedBPs/0Project/Blueprints/Items/coins/coin_100_bp2.coin_100_bp2_C" (Math|Transform|MakeTransform _returnvalue "0, 0, 0" "0.017500,0.017500,0.017500") "Undefined" 0 0))
    (Variables|Default|SetcoinsHolding (- (Variables|Default|GetcoinsHolding) (* 100 (/ (Variables|Default|GetcoinsHolding) 100)))))
  (if (> (/ (Variables|Default|GetcoinsHolding) 50) 0)
    (for _index_3 (range 1 (/ (Variables|Default|GetcoinsHolding) 50))
      (Game|SpawnActorfromClass "/Game/0-Project/0-Blueprints/00-ImportedBPs/0Project/Blueprints/Items/coins/coin_50_BP2.coin_50_BP2_C" (Math|Transform|MakeTransform _returnvalue "0, 0, 0" "0.012500,0.012500,0.012500") "Undefined" 0 0))
    (Variables|Default|SetcoinsHolding (- (Variables|Default|GetcoinsHolding) (* 50 (/ (Variables|Default|GetcoinsHolding) 50)))))
  (if (> (/ (Variables|Default|GetcoinsHolding) 10) 0)
    (for _index_4 (range 1 (/ (Variables|Default|GetcoinsHolding) 10))
      (Game|SpawnActorfromClass "/Game/0-Project/0-Blueprints/00-ImportedBPs/0Project/Blueprints/Items/coins/coin_10_BP.coin_10_BP_C" (Math|Transform|MakeTransform _returnvalue "0, 0, 0" "0.010000,0.010000,0.010000") "Undefined" 0 0))))

(fn StatsUpdate
  (bind _hp_max (Variables|Default|GetHP_Max))
  (bind _hp_current (Variables|Default|GetHP_Current))
  (bind _returnvalue (Math|Conversions|ToFloat(Integer) _hp_current))
  (bind _returnvalue_2 (Math|Conversions|ToFloat(Integer) _hp_max))
  (bind _returnvalue_3 (/ _returnvalue _returnvalue_2))
  (bind _returnvalue_4 (Math|Float|Clamp(Float) _returnvalue_3))
  (bind _asenemy_hp_2 (Utilities|Casting|CastToEnemyHP_2 (UserInterface|GetUserWidgetObject (Variables|Default|GetEnemyHPWidget))))
  (Progress|SetPercent (Variables|/Game/0-Project/0-Blueprints/00-ImportedBPs/Widgets/EnemyHP_2.EnemyHP_2_C|GetHealth_Bar _asenemy_hp_2) _returnvalue_4)
  (Variables|Default|SetHealth_Pct _returnvalue_4)
  (Progress|SetPercent (Variables|/Game/0-Project/0-Blueprints/00-ImportedBPs/Widgets/EnemyHP_2.EnemyHP_2_C|GetStun_Bar _asenemy_hp_2) (Math|Float|Clamp(Float) (/ (Math|Conversions|ToFloat(Integer) 0) (Math|Conversions|ToFloat(Integer) 0)))))