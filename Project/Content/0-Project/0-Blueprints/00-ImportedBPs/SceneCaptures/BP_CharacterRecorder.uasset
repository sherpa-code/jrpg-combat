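; Character recorder actor from the imported scene-capture Blueprints, built to mirror equipped items on a skeletal mesh, but currently inert.
; All events and functions are empty, and the remaining logic is unreachable, with missing cast classes and broken references.
; The orphaned AttachItem and UnAttachItem graphs switch on equipment slot to destroy or spawn item actors, attaching new ones without collision.
; A disconnected EventGraph chain spawns a back-slot weapon.
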(event Custom|updateBPCharRecWeapon)

(event Custom|EquipItem_1)

(event Custom|UnEquipItem_1)

(event EventBeginPlay)

(event Collision|EventActorBeginOverlap
  (params (OtherActor :type Actor%20Object%20Reference)))

(event EventTick
  (params (DeltaSeconds :type Float%20%28single-precision%29)))

(fn ConstructionScript)

(fn UnAttachItem
  (params (ItemInfo :type Boolean)))

(fn AttachItem
  (params (Item%20Info :type Boolean)))