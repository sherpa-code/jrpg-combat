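; GM_Wild is a game mode for wild areas, holding an unfinished random-encounter system.
; BeginPlay only calls its parent, and the EncounterRoll call is disconnected.
; EncounterRoll checks whether a player character overlaps the first encounter area found, then rolls one-in-three odds with no outcome wired.
; Disconnected fragments hold a level-name check, a "! ! !" alert widget and a game-instance switch to a battle level.
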(event EventBeginPlay
  (Utilities|FlowControl|Sequence
    (:then_0
      (|CallParentFunction))
    (:then_1)))

(event EventTick
  (params (DeltaSeconds :type Float%20%28single-precision%29)))

(fn ConstructionScript
  (|CallParentFunction))

(fn EncounterRoll
  (params (Target%20Level%20Wild :type E_Levels_Wild%20Enum :default "NewEnumerator0"))
  (switch Utilities|FlowControl|Switch|SwitchonE_Levels_Wild Target%20Level%20Wild
    (:NewEnumerator0
      ;[1 1 1] Get array of PC actors overlapping Encounter Areas
      (bind _outactors (Actor|GetAllActorsOfClass 0))
      ;[1 1 1] If there are any then...
      (if (> (Utilities|Array|Length (Collision|GetOverlappingActors (Utilities|Array|Get(acopy) _outactors) "/Game/0-Project/0-Blueprints/6-Characters/60-PC/PC_Parent.PC_Parent_C" :!class /Script/Engine.Actor)) 0)
        ;[1 1 1] 1/3 chance for random battle
        (switch int (Math|Random|RandomIntegerinRange 0 2))))))