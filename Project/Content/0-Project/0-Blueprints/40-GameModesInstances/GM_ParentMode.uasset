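; Parent Game Mode that links a level to the shared Reference Manager and records the current level on open.
; Its setup function finds the first actor tagged "Reference Manager", then casts and caches it.
; It then calls the current-level name save on that manager's Game Instance reference, updating the last occupied level.
; No event in this file calls the function, and the debug prints are disconnected.
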(fn ConstructionScript)

(fn SetReferenceMangerRefs(onOpenLevel)
  (Utilities|FlowControl|Sequence
    (:then_0
      ;[0.4948 1 0.4405] Save Reference Manager ref
      (bind _outactors (Actor|GetAllActorswithTag "Reference Manager"))
      (bind _asreference_manager (Utilities|Casting|CastToReference_Manager (Utilities|Array|Get(acopy) _outactors)))
      (bind _output_get (Variables|Default|SetReference%20Manager _asreference_manager)))
    (:then_4
      ;[1 1 1] MyGameInstance: Update Level Last Occupied
      (Default|LevelCurrentNameSave (Variables|/Game/0-Project/0-Blueprints/Reference_Manager.Reference_Manager_C|GetMyGameInstance (Variables|Default|GetReference%20Manager))))))