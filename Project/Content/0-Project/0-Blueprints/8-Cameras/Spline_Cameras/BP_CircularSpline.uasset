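; Circular spline actor in the spline camera set that builds an approximate circle from a radius, with no runtime logic.
; The Construction Script rebuilds four local-space points and sets their tangents using a multiplier derived from the cubic Bézier circle constant plus one.
; It also scales two marker arrows by the radius, placing the green TravelDirection arrow at point zero to face along the spline.
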(event EventBeginPlay)

(event Collision|EventActorBeginOverlap
  (params (OtherActor :type Actor%20Object%20Reference)))

(event EventTick
  (params (DeltaSeconds :type Float%20%28single-precision%29)))

(fn ConstructionScript
  (bind _circle_spline (Variables|Default|GetCircle_Spline))
  (bind _returnvalue (Spline|GetLocationatSplinePoint _circle_spline 0 "World"))
  (Utilities|FlowControl|Sequence
    (:then_0
      ;[1 1 1] Spawn 4 spline nodes to create circle out of
      (Spline|ClearSplinePoints (Variables|Default|GetCircle_Spline) true)
      (Spline|AddSplinePoint (Variables|Default|GetCircle_Spline) (Math|Vector|MakeVector (Variables|Default|GetCircle%20Spline%20Radius) 0.0 0.0) "Local" true)
      (Spline|AddSplinePoint (Variables|Default|GetCircle_Spline) (Math|Vector|MakeVector 0.0 (Variables|Default|GetCircle%20Spline%20Radius) 0.0) "Local" true)
      (Spline|AddSplinePoint (Variables|Default|GetCircle_Spline) (Math|Vector|MakeVector (* (Variables|Default|GetCircle%20Spline%20Radius) -1.0) 0.0 0.0) "Local" true)
      (Spline|AddSplinePoint (Variables|Default|GetCircle_Spline) (Math|Vector|MakeVector 0.0 (* (Variables|Default|GetCircle%20Spline%20Radius) -1.0) 0.0) "Local" true))
    (:then_1
      ;[1 1 1] Circular arc approximation
      (Variables|Default|SetSpline%20Tangent%20Multiplier%20for%20optimal%20approximation%20of%20circle (+ (|((4*((sqrt(2))-1))/3)) 1.0)))
    (:then_2
      ;[1 1 1] Set tangent value for each spline node
      (for _index (range 0 (Spline|GetNumberOfSplinePoints (Variables|Default|GetCircle_Spline)))
        (bind _output_get (Variables|Default|SetCurrent%20Spline%20Number _index))
        (switch int _output_get
          (:0
            (Spline|SetTangentatSplinePoint (Variables|Default|GetCircle_Spline) (Variables|Default|GetCurrent%20Spline%20Number) (Math|Vector|MakeVector 0.0 (* (* (Variables|Default|GetCircle%20Spline%20Radius) (Variables|Default|GetSpline%20Tangent%20Multiplier%20for%20optimal%20approximation%20of%20circle)) 1.0) 0.0) "Local" true))
          (:1
            (Spline|SetTangentatSplinePoint (Variables|Default|GetCircle_Spline) (Variables|Default|GetCurrent%20Spline%20Number) (Math|Vector|MakeVector (* (* (Variables|Default|GetCircle%20Spline%20Radius) (Variables|Default|GetSpline%20Tangent%20Multiplier%20for%20optimal%20approximation%20of%20circle)) -1.0) 0.0 0.0) "Local" true))
          (:2
            (Spline|SetTangentatSplinePoint (Variables|Default|GetCircle_Spline) (Variables|Default|GetCurrent%20Spline%20Number) (Math|Vector|MakeVector 0.0 (* (* (Variables|Default|GetCircle%20Spline%20Radius) (Variables|Default|GetSpline%20Tangent%20Multiplier%20for%20optimal%20approximation%20of%20circle)) -1.0) 0.0) "Local" true))
          (:3
            (Spline|SetTangentatSplinePoint (Variables|Default|GetCircle_Spline) (Variables|Default|GetCurrent%20Spline%20Number) (Math|Vector|MakeVector (* (* (Variables|Default|GetCircle%20Spline%20Radius) (Variables|Default|GetSpline%20Tangent%20Multiplier%20for%20optimal%20approximation%20of%20circle)) 1.0) 0.0 0.0) "Local" true)))))
    (:then_3
      (Utilities|FlowControl|Sequence
        (:then_0
          ;[1 1 1] Scale red arrow relative to desired circle radius
          (Variables|/Script/Engine.ArrowComponent|SetArrowSize (Variables|Default|GetDistance%20Zero) (* (Variables|/Script/Engine.ArrowComponent|GetArrowSize (Variables|Default|GetDistance%20Zero)) (/ (Variables|Default|GetCircle%20Spline%20Radius) 1e+01)))
          ;[1 1 1] Scale green arrow relative to desired circle radius
          (Variables|/Script/Engine.ArrowComponent|SetArrowSize (Variables|Default|GetTravel%20Direction) (* (Variables|/Script/Engine.ArrowComponent|GetArrowSize (Variables|Default|GetTravel%20Direction)) (/ (Variables|Default|GetCircle%20Spline%20Radius) 1e+01))))
        (:then_1
          ;[1 1 1] Place Green starting point at Spline Node Zero and make it point to the positive direction (Direction of travel)
          (Transformation|SetWorldTransform (Variables|Default|GetTravel%20Direction) (Math|Transform|MakeTransform _returnvalue (Math|Rotator|FindLookatRotation _returnvalue (Spline|GetLocationatDistanceAlongSpline _circle_spline 0.01 "World")) "1,1,1") false false))))))