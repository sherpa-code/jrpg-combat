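; AreaDangerLevel1A_BP is an unfinished danger-area actor meant to trigger random battles at Battle Zone A.
; RandomBattleBZA rolls a 50% chance, then casts to MyGameInstance and Magic_Character and sets LevelLastPCTransform on the game instance.
; That transform receives no player value, and the function does not yet start a battle.
; The overlap events are empty, so nothing in this Blueprint calls the function.
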(event EventBeginPlay)

(event Collision|EventActorBeginOverlap
  (params (OtherActor :type Actor%20Object%20Reference)))

(event EventTick
  (params (DeltaSeconds :type Float%20%28single-precision%29)))

(event Collision|EventActorEndOverlap
  (params (OtherActor :type Actor%20Object%20Reference)))

(fn ConstructionScript)

(fn RandomBattle-BZA
  ;[1 1 1] 50% chance to start battle at Battle Zone A when called
  (switch int (Math|Random|RandomIntegerinRange 0 1)
    (:0
      (bind _asmy_game_instance (Utilities|Casting|CastToMyGameInstance (Game|GetGameInstance)))
      (bind _asmagic_character (Utilities|Casting|CastToMagic_Character (Game|GetPlayerCharacter 0)))
      (Variables|/Game/0-Project/0-Blueprints/MyGameInstance.MyGameInstance_C|SetLevel_Last_PC_Transform _asmy_game_instance "" (Transformation|GetWorldLocation (Variables|/Script/Engine.Actor|GetRootComponent _asmagic_character))))))